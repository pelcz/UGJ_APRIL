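; Red enemy pawn that wanders until the player enters its agro trigger, then gives chase.
; Wandering loops AI Move To toward random points around its current location, with random pauses between moves.
; Trigger overlap sets IsChasing to end wandering, changes walk speed, and repeatedly re-issues movement toward the player after successful moves; chasing is never cleared.
; A separate Camera Look At Pawn graph computes a look-at rotation toward Container.
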(event `self.ReceiveBeginPlay`
  ;[1 1 1] Wandering
  (if (not (`self.isChasing`))
    (`|AIMoveTo` self (`NavigationSystem.GetRandomPointInRadius` (`self.K2_GetActorLocation` self) 600.0) :!label _label ; Chase Player
      (:`OnSuccess`
        _)
      (:`OnFail`
        _))
    (`KismetSystemLibrary.Delay` (`KismetMathLibrary.RandomFloatInRange` 0.3 4.0)) ; Move again after random delay
    (if (not (`self.isChasing`))
      (goto _label))))

(event `self.Agro_Trigger.OnComponentBeginOverlap`
  (params (OtherActor :type "Actor Object Reference") (OtherComp :type "PrimitiveComponent Object Reference") (OtherBodyIndex :type Integer) (bFromSweep :type Boolean) (SweepResult :type "EngineTypes.HitResult Structure (by ref)"))
  ;[1 1 1] Chasing
  (bind _asplayer_pawn (cast `/Game/Blueprints/Player_Pawn` OtherActor)) ; Check if player
  (set `self.isChasing` true)
  (set `CharacterMovementComponent.MaxWalkSpeed` 300.0 (`self.CharacterMovement`))
  (`|AIMoveTo` self (0.0 0.0 0.0) _asplayer_pawn :!label _label_2 ; Chase Player
    (:`OnSuccess`
      (`KismetSystemLibrary.Delay` 0.2) ; Keep chasing
      (goto _label_2))))

(fn `UserConstructionScript`)